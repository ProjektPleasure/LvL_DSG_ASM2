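; Weapon pickup that gives the player a sci-fi auto rifle or heavy pistol, chosen by the Weapon enum.
; The construction script maps that choice to the weapon class and skeletal mesh.
; On collection, it runs the parent pickup logic, then passes the class and its default ammo to the weapon component on player pawn 0, regardless of which actor collected it.
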(fn `PickupCollected`
  (params (OtherActor :type "Actor Object Reference"))
  (bind _weaponclass (`self.WeaponClass`))
  (bind _returnvalue (`self.GetComponentByClass` (`GameplayStatics.GetPlayerPawn` 0) "/Game/GameConent/Player/Blueprints/AC_WeaponComponent.AC_WeaponComponent_C"))
  (`parent.PickupCollected` OtherActor)
  (`/Engine/EditorBlueprintResources/StandardMacros.IsValid` _returnvalue
    (:`Is Valid`
      (`/Game/GameConent/Player/Blueprints/AC_WeaponComponent.PickupWeapon` _returnvalue _weaponclass (defaults `Object` _weaponclass)))))

(fn `UserConstructionScript`
  (set `self.WeaponClass` (select `/Game/GameConent/Pickups/E_Weapons` (`self.Weapon`) :`NewEnumerator0` "/Game/0_LevelDesignMechanics/Weapons/LD_Weap_ScifiAutoRifle.LD_Weap_ScifiAutoRifle_C" :`NewEnumerator1` "/Game/0_LevelDesignMechanics/Weapons/LD_Weap_ScifiHeavyPistol.LD_Weap_ScifiHeavyPistol_C" :!type "/Game/GameConent/Weapons/BP_Weapon Class Reference"))
  (`SkeletalMeshComponent.SetSkeletalMeshAsset` (`self.SkeletalMesh`) (select `/Game/GameConent/Pickups/E_Weapons` (`self.Weapon`) :`NewEnumerator0` "/Game/SciFiWeapDark/Weapons/Darkness_AssaultRifle.Darkness_AssaultRifle" :`NewEnumerator1` "/Game/SciFiWeapDark/Weapons/Darkness_Pistol.Darkness_Pistol" :!type "SkeletalMesh Object Reference")))