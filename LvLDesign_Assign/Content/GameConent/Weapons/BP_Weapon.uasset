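; Base weapon Blueprint for the first-person character, handling firing, ammo, recoil and iron sights, with empty ShootProjectile and FireReleased functions.
; Firing with ammo left consumes a round, triggers character recoil and, for projectile weapons, calls ShootProjectile.
; Projectile aim comes from a camera trace within a spray cone, narrowed or widened by iron-sight state, which rotates the spawn point toward the target.
; Ammo changes update a widget, coloured by remaining percentage.
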(event `self.ReceiveBeginPlay`
  (bind _asbp_first_person_character (cast `/Game/GameConent/Player/Blueprints/BP_FirstPersonCharacter` (`self.GetOwner`)))
  (set `self.FPSCharRef` _asbp_first_person_character)
  (bind _asui_ammo (cast `/Game/GameConent/Weapons/UI_Ammo` (`WidgetComponent.GetWidget` (`self.AmmoWidget`))))
  (bind _output_get (set `self.AmmoUI` _asui_ammo))
  (`/Game/GameConent/Weapons/UI_Ammo.UpdateAmmoCount` _output_get (`self.Ammo`))
  (`self.SetAmmoColour`))

(fn `ActivateRecoil`
  (`/Game/GameConent/Player/Blueprints/BP_FirstPersonCharacter.ActivateRecoil` (`self.FPSCharRef`) (`self.Recoil`)))

(fn `AddAmmo`
  (params (Amount :type Integer))
  (bind _output_get (set `self.Ammo` (`KismetMathLibrary.Clamp` (+ (`self.Ammo`) Amount) 0 (`self.MaxAmmo`))))
  (bind _ammoui (`self.AmmoUI`)
    (:`then`
      (`/Game/GameConent/Weapons/UI_Ammo.UpdateAmmoCount` _ammoui _output_get)
      (`self.SetAmmoColour`))
    (:`else`)))

(fn `ConsumeAmmo`
  (bind _result (`/Engine/EditorBlueprintResources/StandardMacros.DecrementInt` (`self.Ammo`))
    (:`  `
      (bind _ammoui (`self.AmmoUI`)
        (:`then`
          (`/Game/GameConent/Weapons/UI_Ammo.UpdateAmmoCount` _ammoui _result)
          (`self.SetAmmoColour`))
        (:`else`)))))

(fn `FirePressed`
  (if (> (`self.Ammo`) 0)
    (`self.SetProjectileSpawnRotation`)
    (`self.ConsumeAmmo`)
    (`self.ActivateRecoil`)
    (if (`self.bUseProjectile`)
      (`self.ShootProjectile`))))

(fn `FireReleased`)

(fn `GetAmmoPercentage`
  (returns (Percentage :type "Float (double-precision)"))
  (return (* (/ (`KismetMathLibrary.Conv_IntToDouble` (`self.Ammo`)) (`KismetMathLibrary.Conv_IntToDouble` (`KismetMathLibrary.Max` (`self.MaxAmmo`) 1))) 100.0)))

(fn `SetAmmo`
  (params (Ammo :type Integer))
  (bind _output_get (set `self.Ammo` Ammo))
  (bind _ammoui (`self.AmmoUI`)
    (:`then`
      (`/Game/GameConent/Weapons/UI_Ammo.UpdateAmmoCount` _ammoui _output_get)
      (`self.SetAmmoColour`))
    (:`else`)))

(fn `SetAmmoColour`
  (`self.SetAmmoIndex`)
  (`/Game/GameConent/Weapons/UI_Ammo.SetColour` (`self.AmmoUI`) (select `int` (`self.AmmoColourIndex`) :`0` (`self.AmmoColourEmpty`) :`1` (`self.AmmoColourLow`) :`2` (`self.AmmoColourHigh`))))

(fn `SetAmmoIndex`
  (returns (Index :type Integer))
  (bind _percentage (`self.GetAmmoPercentage`))
  (if (>= _percentage 50.0)
    (bind _output_get (set `self.AmmoColourIndex` 2))
    (return _output_get)
    (elif (>= _percentage 10.0)
      (bind _output_get_2 (set `self.AmmoColourIndex` 1))
      (return _output_get_2)
      (else
        (bind _output_get_3 (set `self.AmmoColourIndex` 0))
        (return _output_get_3)))))

(fn `SetIronSight`
  (params (bIronSight :type Boolean))
  (bind _returnvalue (`SkeletalMeshComponent.GetAnimInstance` (`/Game/GameConent/Player/Blueprints/BP_FirstPersonCharacter.FirstPersonMesh` (`self.FPSCharRef`))))
  (set `self.bIronSight` bIronSight)
  (`AnimInstance.Montage_Stop` _returnvalue 0.1 (`AnimInstance.GetCurrentActiveMontage` _returnvalue))
  (if (`self.bHideReticleOnIronSight`)
    (set `Widget.Visibility` (select `bool` (`self.bIronSight`) :`false` "Visible" :`true` "Hidden" :!type "ESlateVisibility Enum") (`/Game/GameConent/Player/Blueprints/UI/UI_PlayerHUD.Reticle` (`/Game/GameConent/Player/Blueprints/BP_FirstPersonCharacter.PlayerHUD` (`self.FPSCharRef`))))))

(fn `SetProjectileSpawnRotation`
  (if (`self.bUseProjectile`)
    (bind _fpscharref (`self.FPSCharRef`)
      (:`then`
        (bind _firstpersoncamera (`/Game/GameConent/Player/Blueprints/BP_FirstPersonCharacter.FirstPersonCamera` _fpscharref))
        (bind _returnvalue (`SceneComponent.K2_GetComponentLocation` _firstpersoncamera))
        (bind (_outhit _returnvalue_2) (`KismetSystemLibrary.LineTraceSingle` _returnvalue (+ _returnvalue (* (`KismetMathLibrary.RandomUnitVectorInConeInDegrees` (`SceneComponent.GetForwardVector` _firstpersoncamera) (`KismetMathLibrary.SelectFloat` (`self.IronSightSprayAngle`) (`self.SprayAngle`) (`self.bIronSight`))) (`self.Range`))) "TraceTypeQuery3"))
        (bind (_bblockinghit _binitialoverlap _time _distance _location _impactpoint _normal _impactnormal _physmat _hitactor _hitcomponent _hitbonename _bonename _hititem _elementindex _faceindex _tracestart _traceend) (`GameplayStatics.BreakHitResult` _outhit))
        (`SceneComponent.K2_SetWorldRotation` (`self.SpawnLoc`) (`KismetMathLibrary.FindLookAtRotation` (`SceneComponent.K2_GetComponentLocation` (`self.SpawnLoc`)) (`KismetMathLibrary.SelectVector` _impactpoint _traceend _returnvalue_2)) false false))
      (:`else`))))

(fn `ShootProjectile`)

(fn `UserConstructionScript`
  (set `self.SkeletalMesh` (`SkeletalMeshComponent.GetSkeletalMeshAsset` (`self.SkeletalMeshComponent`)))
  (bind _asui_ammo (cast `/Game/GameConent/Weapons/UI_Ammo` (`WidgetComponent.GetWidget` (`self.AmmoWidget`))))
  (bind _output_get (set `self.AmmoUI` _asui_ammo))
  (`/Game/GameConent/Weapons/UI_Ammo.UpdateAmmoCount` _output_get (`self.Ammo`))
  (`self.SetAmmoColour`))